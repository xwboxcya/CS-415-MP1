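; Enemy actor that damages the player on contact, can be shot for score, and destroys itself five seconds after spawning.
; Its collision overlap takes one health from the player, then either flags death and shows the restart display, or plays a camera shake and removes the enemy.
; A confirmed bullet overlap adds a point to the player's score and destroys both bullet and enemy.
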(event `self.ReceiveBeginPlay`
  (`KismetSystemLibrary.Delay` 5.0)
  (`self.K2_DestroyActor`))

(event `self.enemycollision.OnComponentBeginOverlap`
  (params (OverlappedComponent :type "PrimitiveComponent Object Reference") (OtherActor :type "Actor Object Reference") (OtherComp :type "PrimitiveComponent Object Reference") (OtherBodyIndex :type Integer) (bFromSweep :type Boolean) (SweepResult :type "HitResult Structure (by ref)"))
  (`|ExecutionSequence`
    (:`then_0`
      (bind _asbp_player (cast `/Game/InfiniteMatrix/Blueprints/BP_Player` OtherActor))
      (bind _output_get (set `/Game/InfiniteMatrix/Blueprints/BP_Player.CurrentHealth` (- (`/Game/InfiniteMatrix/Blueprints/BP_Player.CurrentHealth` _asbp_player) 1) _asbp_player))
      (if (<= _output_get 0)
        (set `/Game/InfiniteMatrix/Blueprints/BP_Player.IsDead` true _asbp_player)
        (`/Game/InfiniteMatrix/Blueprints/BP_Player.DIsplayRestart` _asbp_player)
        (else
          (`GameplayStatics.PlayWorldCameraShake` "/Game/InfiniteMatrix/Blueprints/Shake.Shake_C" (`self.K2_GetActorLocation` (`GameplayStatics.GetPlayerPawn` 0)) 0.0 500.0)
          (`self.K2_DestroyActor` :!label _label))))
    (:`then_1`
      (bind _asbp_bullet (cast `/Game/InfiniteMatrix/Blueprints/BP_bullet` OtherActor))
      (if (`PrimitiveComponent.IsOverlappingComponent` (`self.enemycollision`) (`/Game/InfiniteMatrix/Blueprints/BP_bullet.bulletcollision` _asbp_bullet))
        (`|ExecutionSequence`
          (:`then_0`
            (bind _asbp_player_2 (cast `/Game/InfiniteMatrix/Blueprints/BP_Player` (`GameplayStatics.GetPlayerPawn` 0)))
            (set `/Game/InfiniteMatrix/Blueprints/BP_Player.CurrentScore` (+ (`/Game/InfiniteMatrix/Blueprints/BP_Player.CurrentScore` _asbp_player_2) 1) _asbp_player_2))
          (:`then_1`
            (`self.K2_DestroyActor` _asbp_bullet)
            (goto _label)))))))

(fn `UserConstructionScript`)